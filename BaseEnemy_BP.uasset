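; BaseEnemy_BP is an enemy actor for turn-based combat, apparently a base class, with placeholder turn logic.
; Its Box overlap starts combat on BP_MainPC unless that character has CamToggled or CombatEngaged set.
; Tick polls the GM_MainPC game mode's CurrentTurn and calls TurnStart on the matching value.
; TurnStart takes no action beyond waiting briefly, calling SwitchTurn and printing "PlayerTurn".
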(event `self.ReceiveTick`
  (params (DeltaSeconds :type "Float (single-precision)"))
  (bind _asgm_main_pc (cast `/Game/AustinGame/ThirdPersonCharacter/Blueprints/GM_MainPC` (`GameplayStatics.GetGameMode`)))
  (if (`|EnumEquality` (`/Game/AustinGame/ThirdPersonCharacter/Blueprints/GM_MainPC.Current Turn` _asgm_main_pc) "NewEnumerator0")
    (`self.TurnStart`)))

(event `self.Box.OnComponentBeginOverlap`
  (params (OverlappedComponent :type "PrimitiveComponent Object Reference") (OtherActor :type "Actor Object Reference") (OtherComp :type "PrimitiveComponent Object Reference") (OtherBodyIndex :type Integer) (bFromSweep :type Boolean) (SweepResult :type "HitResult Structure (by ref)"))
  (bind _asbp_main_pc (cast `/Game/AustinGame/ThirdPersonCharacter/Blueprints/BP_MainPC` OtherActor))
  (if (`/Game/AustinGame/ThirdPersonCharacter/Blueprints/BP_MainPC.CamToggled?` _asbp_main_pc)
    _
    (elif (not (`/Game/AustinGame/ThirdPersonCharacter/Blueprints/BP_MainPC.CombatEngaged?` _asbp_main_pc))
      (`/Game/AustinGame/ThirdPersonCharacter/Blueprints/BP_MainPC.Initiate Combat Event` _asbp_main_pc false))))

(event `TurnStart`
  (`KismetSystemLibrary.Delay` 2.0)
  (bind _asgm_main_pc (cast `/Game/AustinGame/ThirdPersonCharacter/Blueprints/GM_MainPC` (`GameplayStatics.GetGameMode`)))
  (`/Game/AustinGame/ThirdPersonCharacter/Blueprints/GM_MainPC.SwitchTurn` _asgm_main_pc)
  (`KismetSystemLibrary.PrintString` "PlayerTurn"))

(fn `UserConstructionScript`)