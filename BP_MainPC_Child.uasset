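; BP_MainPC_Child is a free-moving camera pawn, apparently a BP_MainPC child, used as a toggled camera with its own combat menu.
; On BeginPlay it copies known spells from its instigator BP_MainPC, rebuilds the combat menu and copies combat state.
; Input moves it vertically, and right-click clears the selected spell.
; Toggle, CamDestroy or CombatEnd repossess the instigator and destroy the camera; CombatEnd also calls EndCombat on the instigator.
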(event `self.ReceiveBeginPlay`
  (`parent.ReceiveBeginPlay`)
  (bind _asbp_main_pc (cast `/Game/AustinGame/ThirdPersonCharacter/Blueprints/BP_MainPC` (`self.GetInstigator`)))
  (set `self.SpellsKnown` (`/Game/AustinGame/ThirdPersonCharacter/Blueprints/BP_MainPC.SpellsKnown` _asbp_main_pc))
  (`WidgetLayoutLibrary.RemoveAllWidgets`)
  (bind _returnvalue (`|CreateWidget` "/Game/AustinGame/ThirdPersonCharacter/UI/CombatUI/PlayerCombatMenu_W.PlayerCombatMenu_W_C"))
  (bind _output_get (set `self.CombatMenu Ref` _returnvalue))
  (set `/Game/AustinGame/ThirdPersonCharacter/UI/CombatUI/PlayerCombatMenu_W.IsCamPossessed?` true _output_get)
  (`UserWidget.AddToViewport` (`self.CombatMenu Ref`) 0)
  (set `self.CombatEngaged?` (`/Game/AustinGame/ThirdPersonCharacter/Blueprints/BP_MainPC.CombatEngaged?` (`self.Char Ref`)))
  (set `self.CamToggled?` true))

(event `EnhancedInput|/Game/AustinGame/ThirdPersonCharacter/input/IA_ToggleCamera`
  (params (ActionValue :type Boolean) (ElapsedSeconds :type "Float (double-precision)") (TriggeredSeconds :type "Float (double-precision)") (InputAction :type "InputAction Object Reference" :default "/Game/AustinGame/ThirdPersonCharacter/input/IA_ToggleCamera.IA_ToggleCamera"))
  (bind _returnvalue (`self.GetInstigator`))
  (:`Triggered`
    (`/Engine/EditorBlueprintResources/StandardMacros.IsValid` _returnvalue :!label _label
      (:`Is Valid`
        (`Controller.Possess` (`GameplayStatics.GetPlayerController` 0) _returnvalue)
        (`self.K2_DestroyActor`)
        (bind _asbp_main_pc (cast `/Game/AustinGame/ThirdPersonCharacter/Blueprints/BP_MainPC` (`GameplayStatics.GetPlayerCharacter` 0)))
        (set `/Game/AustinGame/ThirdPersonCharacter/Blueprints/BP_MainPC.CamToggled?` false _asbp_main_pc)
        (set `/Game/AustinGame/ThirdPersonCharacter/UI/CombatUI/PlayerCombatMenu_W.IsCamPossessed?` false (`self.CombatMenu Ref`))
        (`KismetSystemLibrary.PrintString` "cam toggled")))))

(event `CamDestroy`
  (goto _label))

(event `CombatEnd`
  (bind _returnvalue (`self.GetInstigator`))
  (`/Engine/EditorBlueprintResources/StandardMacros.IsValid` _returnvalue
    (:`Is Valid`
      (`Controller.Possess` (`GameplayStatics.GetPlayerController` 0) _returnvalue)
      (`self.K2_DestroyActor`)
      (bind _asbp_main_pc (cast `/Game/AustinGame/ThirdPersonCharacter/Blueprints/BP_MainPC` (`GameplayStatics.GetPlayerCharacter` 0)))
      (set `/Game/AustinGame/ThirdPersonCharacter/Blueprints/BP_MainPC.CamToggled?` false _asbp_main_pc)
      (set `/Game/AustinGame/ThirdPersonCharacter/UI/CombatUI/PlayerCombatMenu_W.IsCamPossessed?` false (`self.CombatMenu Ref`))
      (`KismetSystemLibrary.PrintString` "cam toggled")
      (bind _asbp_main_pc_2 (cast `/Game/AustinGame/ThirdPersonCharacter/Blueprints/BP_MainPC` _returnvalue))
      (set `/Game/AustinGame/ThirdPersonCharacter/Blueprints/BP_MainPC.CamToggled?` false _asbp_main_pc_2)
      (set `/Game/AustinGame/ThirdPersonCharacter/Blueprints/BP_MainPC.IsCamPossessed?` false _asbp_main_pc_2)
      (`self.EndCombat` _asbp_main_pc_2))))

(event `EnhancedInput|/Game/AustinGame/ThirdPersonCharacter/input/IA_CameraAscend`
  (params (ActionValue :type Boolean) (ElapsedSeconds :type "Float (double-precision)") (TriggeredSeconds :type "Float (double-precision)") (InputAction :type "InputAction Object Reference" :default "/Game/AustinGame/ThirdPersonCharacter/input/IA_CameraAscend.IA_CameraAscend"))
  (:`Triggered`
    (`self.AddMovementInput` (`SceneComponent.GetUpVector` (`self.CapsuleComponent`)) 0.87)))

(event `EnhancedInput|/Game/AustinGame/ThirdPersonCharacter/input/IA_CameraDescend`
  (params (ActionValue :type Boolean) (ElapsedSeconds :type "Float (double-precision)") (TriggeredSeconds :type "Float (double-precision)") (InputAction :type "InputAction Object Reference" :default "/Game/AustinGame/ThirdPersonCharacter/input/IA_CameraDescend.IA_CameraDescend"))
  (:`Triggered`
    (`self.AddMovementInput` (`SceneComponent.GetUpVector` (`self.CapsuleComponent`)) -0.87)))

(event `Key|RightMouseButton`
  (params (Key :type "Key Structure"))
  (:`Pressed`
    (set `self.SpellSelected` (struct))))

(fn `UserConstructionScript`
  (`parent.UserConstructionScript`))