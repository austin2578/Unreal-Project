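; Base interactable pickup actor that hands its item to the player character when interacted with.
; The construction script fills ItemInfo from the ItemInfo_DT data table, using the ItemName enum converted to a row name.
; Interact casts the player character to BP_MainPC, calls PickupItem with that info, then destroys the actor after a very short delay.
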(event `/Game/AustinGame/ThirdPersonCharacter/InventorySystem/Interact_BPI.Interact`
  (bind _asbp_main_pc (cast `/Game/AustinGame/ThirdPersonCharacter/Blueprints/BP_MainPC` (`GameplayStatics.GetPlayerCharacter` 0)))
  (`/Game/AustinGame/ThirdPersonCharacter/Blueprints/BP_MainPC.PickupItem` _asbp_main_pc (`self.ItemInfo`))
  (`KismetSystemLibrary.Delay` 0.01)
  (`self.K2_DestroyActor`))

(fn `UserConstructionScript`
  ;[1 1 1] Set item values based off of data table
  (bind _returnvalue (`|GetDataTableRow` "/Game/AustinGame/ThirdPersonCharacter/InventorySystem/ItemInfo_DT.ItemInfo_DT" (`KismetStringLibrary.Conv_StringToName` (`|GetEnumeratorNameAsString` (`self.ItemName`))))
    (:`then`
      (set `self.ItemInfo` _returnvalue))))