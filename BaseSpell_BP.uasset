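; BaseSpell_BP is a spell projectile base that configures itself from the Spells_DT data table.
; Its construction script converts the SpellName enum in SpellInfo to a row name and copies the found row back into SpellInfo.
; That row's Speed sets both initial and max speed on ProjectileMovement.
; The gravity scale assignment is unconnected and never runs, and the event graph holds only disabled placeholder events.
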(fn `UserConstructionScript`
  (bind _projectilemovement (`self.ProjectileMovement`))
  (bind _returnvalue (`|GetDataTableRow` "/Game/AustinGame/ThirdPersonCharacter/Blueprints/MagicSystem/Spells_DT.Spells_DT" (`KismetStringLibrary.Conv_StringToName` (`|GetEnumeratorNameAsString` (`.SpellName_10_71668BE34663BBE95C6A8097C21F926A` (break `/Game/AustinGame/ThirdPersonCharacter/Blueprints/MagicSystem/SpellInfo_S` (`self.SpellInfo`))))))
    (:`then`
      (bind _output_get (set `self.SpellInfo` _returnvalue))
      (bind (_spellclass _spellname _spelltype _spellimage _spellelement _manacost _potency _price _speed _gravityscale) (break `/Game/AustinGame/ThirdPersonCharacter/Blueprints/MagicSystem/SpellInfo_S` _output_get))
      (set `ProjectileMovementComponent.InitialSpeed` _speed _projectilemovement)
      (set `ProjectileMovementComponent.MaxSpeed` _speed _projectilemovement))))